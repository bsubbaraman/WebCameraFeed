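; CameraPlane_BP is an actor that shows a live device camera feed on a plane mesh.
; On BeginPlay it creates a dynamic instance of the M_CamChroma_0 material on the plane and feeds it the WebCamera component's texture, switching to the front camera on iOS and Android.
; Tick re-assigns the camera texture to the material every frame so the displayed image follows the feed.
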(event EventBeginPlay
  (bind _returnvalue (Game|GetPlatformName))
  (bind _webcamera (Variables|Default|GetWebCamera))
  (bind _returnvalue_2 (Class|WebCameraComponent|GetTexture (Variables|Default|GetWebCamera)))
  (bind _returnvalue_3 (Rendering|Material|CreateDynamicMaterialInstance (Variables|Default|GetPlane) 0 "/Game/Materials/M_CamChroma_0.M_CamChroma_0" "None" :!class /Script/Engine.PrimitiveComponent))
  (bind _output_get (Variables|Default|SetCurrentMaterialInstance _returnvalue_3))
  (Rendering|Material|SetTextureParameterValue _output_get "Texture" _returnvalue_2)
  (if (or (Utilities|Enum|Equal(Enum) _returnvalue "IOS") (Utilities|Enum|Equal(Enum) _returnvalue "Android"))
    (bind _returnvalue_4 (Class|WebCameraComponent|GetFrontCameraId _webcamera))
    (Class|WebCameraComponent|SetDeviceId _webcamera _returnvalue_4)))

(event Collision|EventActorBeginOverlap
  (params (OtherActor :type Actor%20Object%20Reference)))

(event EventTick
  (params (DeltaSeconds :type Float%20%28single-precision%29))
  (bind _returnvalue (Class|WebCameraComponent|GetTexture (Variables|Default|GetWebCamera)))
  (Rendering|Material|SetTextureParameterValue (Variables|Default|GetCurrentMaterialInstance) "Texture" _returnvalue))

(fn ConstructionScript)